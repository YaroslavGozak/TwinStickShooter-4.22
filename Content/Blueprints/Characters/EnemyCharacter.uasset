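; Enemy character for a twin-stick shooter that damages the hero on contact and may drop a pickup on death.
; Overlapping the hero starts a looping damage timer paced by attack rate; ending overlap clears it.
; AffectHealth handles death: it disables key collisions, adds score through TwinStickMode, detaches the controller, then after a delay destroys itself and randomly spawns aid or ammo.
; The construction script tints the body through a dynamic material; explosion spawning is disconnected.
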(event `/Game/Blueprints/IDamageble.AffectHealth`
  (params (Delta :type "Float (single-precision)"))
  (bind _capsulecomponent (`self.CapsuleComponent`))
  (bind _damagevolume (`self.DamageVolume`))
  (`self.CalculateHealth` Delta)
  (if (`self.IsDead`)
    (`PrimitiveComponent.SetCollisionResponseToChannel` _capsulecomponent "ECC_WorldDynamic" "ECR_Ignore")
    (`PrimitiveComponent.SetCollisionResponseToChannel` _capsulecomponent "ECC_Pawn" "ECR_Ignore")
    (`PrimitiveComponent.SetCollisionResponseToChannel` _damagevolume "ECC_WorldDynamic" "ECR_Ignore")
    (`PrimitiveComponent.SetCollisionResponseToChannel` _damagevolume "ECC_Pawn" "ECR_Ignore")
    (bind _astwin_stick_mode (cast `/Game/Blueprints/Gameplay/TwinStickMode` (`GameplayStatics.GetGameMode`)))
    (`/Game/Blueprints/Gameplay/TwinStickMode.IncrementScore` _astwin_stick_mode (`self.Score`))
    (`self.DetachFromControllerPendingDestroy`)
    (`KismetSystemLibrary.Delay` (`self.TimeBeforeDestroy`))
    (bind _output_get (set `self.EnemyDeathPosition` (`self.GetTransform`)))
    (`self.K2_DestroyActor`)
    (`self.TrySpawnPickup`)))

(event `self.ReceiveActorBeginOverlap`
  (params (OtherActor :type "Actor Object Reference"))
  (bind _ashero_character_white (cast `/Game/Blueprints/Characters/HeroCharacterWhite` OtherActor))
  (set `self.Hero` _ashero_character_white)
  (`KismetSystemLibrary.K2_SetTimer` null "DamageTheHero" (/ 1.0 (`self.AttacksPerSecond`)) true))

(event `self.ReceiveActorEndOverlap`
  (params (OtherActor :type "Actor Object Reference"))
  (if (== OtherActor (`self.Hero`))
    (`KismetSystemLibrary.K2_ClearTimer` null "DamageTheHero")))

(event `DamageTheHero`
  (`/Game/Blueprints/Characters/HeroCharacterWhite.AffectHealth` (`self.Hero`) (`self.Damage`)))

(event `TrySpawnPickup`
  (bind _returnvalue (`KismetMathLibrary.RandomInteger` 20))
  (bind _enemydeathposition (`self.EnemyDeathPosition`))
  (if (> _returnvalue 8)
    (if (> _returnvalue 12)
      (`|SpawnActorFromClass` "/Game/Blueprints/AidPickup.AidPickup_C" _enemydeathposition "Undefined" "OverrideRootScale" null null)
      (else
        (`|SpawnActorFromClass` "/Game/Blueprints/AmmoPickup.AmmoPickup_C" _enemydeathposition "Undefined" "OverrideRootScale" null null)))))

(event `SpawnAmmo`
  (`|SpawnActorFromClass` "/Game/Blueprints/AmmoPickup.AmmoPickup_C" (`self.EnemyDeathPosition`) "Undefined" "OverrideRootScale" null null))

(fn `UserConstructionScript`
  (bind _returnvalue (`PrimitiveComponent.CreateDynamicMaterialInstance` (`self.Mesh`) 0 null "None"))
  (bind _output_get (set `self.NewVar_0_0` _returnvalue))
  (`MaterialInstanceDynamic.SetVectorParameterValue` _output_get "BodyColor" (`self.EnemyColor`)))