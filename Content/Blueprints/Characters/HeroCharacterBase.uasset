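; Base twin-stick hero character that moves on world axes, aims, fires, collects health and ammo pickups, and respawns after death.
; BeginPlay attaches a spawned weapon to the hand mesh's gun socket, saves the spawn transform to TwinStickMode and creates the HUD.
; A MouseController aims by screen-space cursor offset and fires by trigger; other controllers' look input both rotates and auto-fires.
; Death disables input, then after a delay requests respawn and destroys character and weapon.
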(event `InputAxis|PullTrigger`
  (params (AxisValue :type "Float (single-precision)"))
  (bind _weapon (`self.Weapon`))
  ;[1 1 1] Mouse Fire
  (cast `/Game/Blueprints/Gameplay/MouseController` (`GameplayStatics.GetPlayerController` 0))
  (`KismetSystemLibrary.PrintString` (`KismetStringLibrary.Conv_DoubleToString` AxisValue))
  (if (> AxisValue 0.0)
    (`/Game/Blueprints/Weapon/Weapon.PullTrigger` _weapon)
    (else
      (`/Game/Blueprints/Weapon/Weapon.ReleaseTrigger` _weapon))))

(event `InputAxisKey|MouseY`
  (params (AxisValue :type "Float (single-precision)"))
  (bind _screenlocation (`PlayerController.ProjectWorldLocationToScreen` (`GameplayStatics.GetPlayerController` 0) (`self.K2_GetActorLocation`) false))
  (bind (_locationx _locationy) (`PlayerController.GetMousePosition` (`GameplayStatics.GetPlayerController` 0)))
  ;[1 1 1] Mouse Rotation
  (cast `/Game/Blueprints/Gameplay/MouseController` (`GameplayStatics.GetPlayerController` 0))
  (`Controller.SetControlRotation` (`self.GetController`) (`KismetMathLibrary.Conv_VectorToRotator` (`KismetMathLibrary.RotateAngleAxis` (`KismetMathLibrary.MakeVector` (- _locationx (`KismetMathLibrary.BreakVector2D` _screenlocation)) (- _locationy (`.Y` (`KismetMathLibrary.BreakVector2D` _screenlocation)))) 90.0 (`self.GetActorUpVector`)))))

(event `InputAxis|LookRight`
  (params (AxisValue :type "Float (single-precision)"))
  (bind _weapon (`self.Weapon`))
  ;[1 1 1] Rotation Key
  (cast `/Game/Blueprints/Gameplay/MouseController` (`GameplayStatics.GetPlayerController` 0)
    (:`CastFailed`
      (bind _returnvalue (`KismetMathLibrary.MakeVector` (stale `InputAxis|LookUp` AxisValue) AxisValue))
      (if (> (`KismetMathLibrary.VSize` _returnvalue) 0.25)
        (`Controller.SetControlRotation` (`self.GetController`) (`KismetMathLibrary.Conv_VectorToRotator` _returnvalue))
        (`/Game/Blueprints/Weapon/Weapon.PullTrigger` _weapon)
        (else
          (`/Game/Blueprints/Weapon/Weapon.ReleaseTrigger` _weapon))))))

(event `InputAxis|LookUp`
  (params (AxisValue :type "Float (single-precision)"))
  ;[1 1 1] Rotation Key
)

(event `self.ReceiveBeginPlay`
  (bind _mesh (`self.Mesh`))
  (`|ExecutionSequence`
    (:`then_0`
      ;[1 1 1] Weapon Setup
      (bind _returnvalue (`|SpawnActorFromClass` "/Game/Blueprints/Weapon/Weapon.Weapon_C" (`SceneComponent.K2_GetComponentToWorld` _mesh) "Undefined" "OverrideRootScale" null null))
      (bind _output_get (set `self.Weapon` _returnvalue))
      (`self.K2_AttachToComponent` _output_get _mesh "GunSocket" "SnapToTarget" "SnapToTarget" "KeepWorld" true))
    (:`then_1`
      ;[1 1 1] Push Transform to GameMode
      (bind _astwin_stick_mode (cast `/Game/Blueprints/Gameplay/TwinStickMode` (`GameplayStatics.GetGameMode`)))
      (bind _output_get_2 (set `self.GameMode` _astwin_stick_mode))
      (set `/Game/Blueprints/Gameplay/TwinStickMode.PlayerSpawnTransform` (`self.GetTransform`) _output_get_2))
    (:`then_2`
      (bind _returnvalue_2 (`|CreateWidget` "/Game/Blueprints/TwinStickHud.TwinStickHud_C"))
      (`UserWidget.AddToViewport` _returnvalue_2 0))))

(event `InputAxis|MoveUp`
  (params (AxisValue :type "Float (single-precision)"))
  ;[1 1 1] Movement
  (`self.AddMovementInput` (1.0 0.0 0.0) AxisValue))

(event `InputAxis|MoveRight`
  (params (AxisValue :type "Float (single-precision)"))
  ;[1 1 1] Movement
  (`self.AddMovementInput` (0.0 1.0 0.0) AxisValue))

(event `/Game/Blueprints/IDamageble.AffectHealth`
  (params (Delta :type "Float (single-precision)"))
  ;[1 1 1] Health
  (`self.CalculateHealth` Delta)
  (if (`self.IsDead`)
    (`self.DisableInput` null)
    (`/Game/Blueprints/Weapon/Weapon.ReleaseTrigger` (`self.Weapon`))
    (`KismetSystemLibrary.Delay` 3.0)
    (`/Game/Blueprints/Gameplay/TwinStickMode.RespawnPlayer` (`self.GameMode`))
    (`self.K2_DestroyActor` self)
    (`self.K2_DestroyActor` (`self.Weapon`))))

(event `Key|R`
  (params (Key :type "Key Structure"))
  ;[1 1 1] Reload Key
  (:`Pressed`
    (`/Game/Blueprints/Weapon/Weapon.Reload` (`self.Weapon`))))

(event `self.ReceiveActorBeginOverlap`
  (params (OtherActor :type "Actor Object Reference"))
  (bind _weapon (`self.Weapon`))
  ;[1 1 1] Pickup
  (bind _asaid_pickup (cast `/Game/Blueprints/AidPickup` OtherActor)
    (:`then`
      (`/Game/Blueprints/IDamageble.AffectHealth` (`/Game/Blueprints/AidPickup.Health` _asaid_pickup))
      (`self.K2_DestroyActor` _asaid_pickup))
    (:`CastFailed`
      (bind _asammo_pickup (cast `/Game/Blueprints/AmmoPickup` OtherActor))
      (`/Game/Blueprints/Weapon/Weapon.SetRoundsLeft` _weapon (+ (`/Game/Blueprints/AmmoPickup.Rounds` _asammo_pickup) (`/Game/Blueprints/Weapon/Weapon.RoundsLeft` _weapon)))
      (`self.K2_DestroyActor` _asammo_pickup))))

(event `InputAction|Pause` :paused true
  (params (Key :type "Key Structure"))
  ;[1 1 1] Pause the Game
)

(fn `UserConstructionScript`)