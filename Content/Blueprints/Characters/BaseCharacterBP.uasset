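; Base character Blueprint that tracks health and death state.
; CalculateHealth adds a signed delta to Health, capping it at MaxHealth with no lower clamp, then calls CalculateDead.
; CalculateDead sets IsDead whenever Health is at or below zero and clears it otherwise, so regaining health undoes death.
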(event `CalculateHealth`
  (params (Delta :type "Float (double-precision)"))
  (bind _returnvalue (+ Delta (`self.Health`)))
  (if (<= _returnvalue (`self.MaxHealth`))
    (set `self.Health` _returnvalue)
    (else
      (set `self.Health` (`self.MaxHealth`))))
  (`self.CalculateDead`))

(event `CalculateDead`
  (if (<= (`self.Health`) 0.0)
    (set `self.IsDead` true)
    (else
      (set `self.IsDead` false))))

(fn `UserConstructionScript`)