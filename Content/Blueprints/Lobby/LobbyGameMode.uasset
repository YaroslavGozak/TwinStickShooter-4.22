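; Lobby game mode that runs a twin-stick shooter session, tracking score, ammo and player respawn.
; On BeginPlay it starts a looping SpawnEnemy timer on the first EnemySpawner, with production mode adding a delay and music.
; Respawn destroys all enemies and possesses a new hero.
; Pause functions toggle menu or HUD, input mode, cursor and music; character-swap, update and launch events are empty stubs.
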(event `RespawnPlayer`
  (bind _outactors (`GameplayStatics.GetAllActorsOfClass` "/Game/Blueprints/Characters/EnemyCharacter.EnemyCharacter_C"))
  (for _array_element _outactors
    (`self.K2_DestroyActor` _array_element))
  (bind _returnvalue (`|SpawnActorFromClass` "/Game/Blueprints/Characters/HeroCharacter.HeroCharacter_C" (`self.PlayerSpawnTransform`) "Undefined" "OverrideRootScale" null null))
  (`Controller.Possess` (`GameplayStatics.GetPlayerController` 0) _returnvalue))

(event `self.ReceiveBeginPlay`
  (`|ExecutionSequence`
    (:`then_0`
      (if (`self.EnableProdMode`)
        (`KismetSystemLibrary.Delay` 10.0))
      (bind _outactors (`GameplayStatics.GetAllActorsOfClass` "/Game/Blueprints/EnemySpawner.EnemySpawner_C"))
      (bind _output_get (set `self.EnemySpawner` (`|GetArrayItem` _outactors)))
      (`KismetSystemLibrary.K2_SetTimer` _output_get "SpawnEnemy" (/ 1.0 (`self.Enemies per second`)) true))
    (:`then_1`
      (if (`self.EnableProdMode`)
        (bind _returnvalue (`GameplayStatics.SpawnSound2D` "/Game/Sounds/Rammstein_-_Engel.Rammstein_-_Engel" 1.0 1.0 0.0 null))
        (set `self.EmbientSound` _returnvalue)))))

(event `IncrementScore`
  (params (DeltaScore :type Integer))
  (set `self.Score` (+ DeltaScore (`self.Score`))))

(event `SetRoundsLeft`
  (params (Rounds :type Integer))
  (set `self.RoundsLeft` Rounds))

(event `SetRoundsInMagazine`
  (params (Rounds :type Integer))
  (set `self.RoundsInMagazine` Rounds))

(event `PauseMusic`
  (`AudioComponent.SetPaused` (`self.EmbientSound`) true))

(event `UnpauseMusic`
  (`AudioComponent.SetPaused` (`self.EmbientSound`) false))

(event `SwapCharacter`
  (params (PlayerController :type "PlayerController Object Reference") (CharacterClass :type "Character Class Reference") (ChangedStatus :type Boolean)))

(event `EveryoneUpdate`)

(event `LaunchTheGame`)

(fn `PauseGame`
  (bind _returnvalue (`GameplayStatics.GetPlayerController` 0))
  (`GameplayStatics.SetGamePaused` true)
  (`/Engine/EditorBlueprintResources/StandardMacros.IsValid` (`self.PauseMenu`)
    (:`Is Valid`
      _)
    (:`Is Not Valid`
      (bind _returnvalue_2 (`|CreateWidget` "/Game/Blueprints/PauseMenu.PauseMenu_C" (`GameplayStatics.GetPlayerController` 0)))
      (set `self.PauseMenu` _returnvalue_2)))
  (`UserWidget.AddToViewport` (`self.PauseMenu`) 0)
  (`WidgetBlueprintLibrary.SetInputMode_UIOnlyEx` (`GameplayStatics.GetPlayerController` 0) (`self.PauseMenu`))
  (set `PlayerController.CurrentMouseCursor` "Default" _returnvalue)
  (set `PlayerController.bShowMouseCursor` true _returnvalue)
  (cast `/Game/Blueprints/Lobby/LobbyGameMode` (`GameplayStatics.GetGameMode`))
  (`self.PauseMusic`))

(fn `UnpauseGame`
  (bind _returnvalue (`GameplayStatics.GetPlayerController` 0))
  (bind _returnvalue_2 (`GameplayStatics.GetPlayerController` 0))
  (`GameplayStatics.SetGamePaused` false)
  (`WidgetLayoutLibrary.RemoveAllWidgets`)
  (`WidgetBlueprintLibrary.SetInputMode_GameOnly` _returnvalue_2)
  (cast `/Game/Blueprints/Gameplay/MouseController` _returnvalue_2
    (:`then`
      _)
    (:`CastFailed`
      (set `PlayerController.bShowMouseCursor` false _returnvalue)))
  (set `PlayerController.CurrentMouseCursor` "Crosshairs" _returnvalue)
  (bind _aslobby_game_mode (cast `/Game/Blueprints/Lobby/LobbyGameMode` (`GameplayStatics.GetGameMode`)))
  (`self.UnpauseMusic` _aslobby_game_mode)
  (`/Engine/EditorBlueprintResources/StandardMacros.IsValid` (`self.TwinStickHud`)
    (:`Is Valid`
      _)
    (:`Is Not Valid`
      (bind _returnvalue_3 (`|CreateWidget` "/Game/Blueprints/TwinStickHud.TwinStickHud_C" (`GameplayStatics.GetPlayerController` 0)))
      (bind _output_get (set `self.TwinStickHud` _returnvalue_3))))
  (`UserWidget.AddToViewport` _output_get 0))

(fn `UserConstructionScript`)