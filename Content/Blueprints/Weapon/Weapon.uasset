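; Twin-stick weapon actor that handles automatic projectile fire, ammo and reloading.
; Pulling the trigger fires once and starts a looping fire-rate timer, guarded by a DoOnce until release.
; Each shot spawns the projectile class selected in GameInfoInstance player data, and an empty magazine triggers a delayed reload from reserve rounds.
; Ammo changes are pushed to TwinStickMode to keep its round counts in sync.
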(event `UpdateGameMode`
  ;[1 1 1] Update Game Mode
  (`/Game/Blueprints/Gameplay/TwinStickMode.SetRoundsLeft` (`self.CurrentGameMode`) (`self.RoundsLeft`))
  (`/Game/Blueprints/Gameplay/TwinStickMode.SetRoundsInMagazine` (`self.CurrentGameMode`) (`self.RoundsInMagazine`)))

(event `self.ReceiveBeginPlay`
  ;[1 1 1] Initialize Weapon
  (set `self.IsReloading` false)
  (bind _astwin_stick_mode (cast `/Game/Blueprints/Gameplay/TwinStickMode` (`GameplayStatics.GetGameMode`)))
  (set `self.CurrentGameMode` _astwin_stick_mode)
  (`self.UpdateGameMode`)
  (bind _asgame_info_instance (cast `/Game/Blueprints/AllLevels/GameInfoInstance` (`GameplayStatics.GetGameInstance`)))
  (set `self.Projectile` (`.Projectile_6_5DA6D52D4B693A26864ED6B9C96EAB02` (break `/Game/Blueprints/AllLevels/ProjectileSelection` (`.MyPlayerProjectileSelection_23_91B97D2A42D5BA4F85578F8D8161D301` (break `/Game/Blueprints/AllLevels/PlayerInfo` (`/Game/Blueprints/AllLevels/GameInfoInstance.PlayerData` _asgame_info_instance)))))))

(event `PullTrigger`
  ;[1 1 1] Handle trigger
  (`/Engine/EditorBlueprintResources/StandardMacros.DoOnce` false :!label _label
    (:`Completed`
      (`self.Fire`)
      (`KismetSystemLibrary.K2_SetTimer` null "Fire" (/ 1.0 (`self.RoundsPerSecond`)) true))))

(event `ReleaseTrigger`
  ;[1 1 1] Handle trigger
  (`KismetSystemLibrary.K2_ClearTimer` null "Fire")
  (goto _label :!via `Reset`))

(event `Fire`
  ;[1 1 1] Fire
  (if (not (`self.IsReloading`))
    (if (> (`self.RoundsInMagazine`) 0)
      (`self.GetProjectile`)
      (`GameplayStatics.PlaySound2D` "/Game/Sounds/silencer4a_Cue.silencer4a_Cue" 3.0 1.0 0.0 null null)
      (`|SpawnActorFromClass` (`self.Projectile`) (`SceneComponent.K2_GetComponentToWorld` (`self.ProjectileSpawnPoint`)) "Undefined" "OverrideRootScale" null null)
      (bind _result (`/Engine/EditorBlueprintResources/StandardMacros.DecrementInt` (`self.RoundsInMagazine`))
        (:`  `
          (set `self.RoundsInMagazine` _result)
          (`self.UpdateGameMode`)))
      (elif (> (`self.RoundsLeft`) 0)
        (`self.Reload`)))))

(event `GetProjectile`
  ;[1 1 1] Get Projectile
  (bind _asgame_info_instance (cast `/Game/Blueprints/AllLevels/GameInfoInstance` (`GameplayStatics.GetGameInstance`)))
  (set `self.Projectile` (`.Projectile_6_5DA6D52D4B693A26864ED6B9C96EAB02` (break `/Game/Blueprints/AllLevels/ProjectileSelection` (`.MyPlayerProjectileSelection_23_91B97D2A42D5BA4F85578F8D8161D301` (break `/Game/Blueprints/AllLevels/PlayerInfo` (`/Game/Blueprints/AllLevels/GameInfoInstance.PlayerData` _asgame_info_instance)))))))

(event `Reload`
  ;[1 1 1] Reload
  (if (not (`self.IsReloading`))
    (if (> (`self.RoundsLeft`) 0)
      (set `self.IsReloading` true)
      (if (>= (`self.RoundsLeft`) (`self.MagazineCapacity`))
        (set `self.RoundsToReload` (`self.MagazineCapacity`))
        (else
          (set `self.RoundsToReload` (`self.RoundsLeft`))))
      (`GameplayStatics.PlaySound2D` "/Game/Sounds/ReloadSound_1.ReloadSound_1" 3.0 1.0 0.0 null null)
      (`KismetSystemLibrary.Delay` (`self.ReloadDuration`))
      (`self.SetRoundsLeft` (+ (- (`self.RoundsLeft`) (`self.RoundsToReload`)) (`self.RoundsInMagazine`)))
      (`self.SetRoundsInMagazine` (`self.RoundsToReload`))
      (set `self.IsReloading` false))))

(event `SetRoundsLeft`
  (params (Rounds :type Integer))
  ;[1 1 1] Managing rounds display and calculation
  (set `self.RoundsLeft` Rounds)
  (`self.UpdateGameMode`))

(event `SetRoundsInMagazine`
  (params (Rounds :type Integer))
  ;[1 1 1] Managing rounds display and calculation
  (set `self.RoundsInMagazine` Rounds)
  (`self.UpdateGameMode`))

(fn `UserConstructionScript`)